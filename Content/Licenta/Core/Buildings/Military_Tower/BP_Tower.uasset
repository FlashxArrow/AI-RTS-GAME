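; BP_Tower is a selectable military tower building whose soldier automatically fires on hostile units.
; A looping timer sphere-traces nearby pawns, and GetClosestEnemy keeps the last hostile within ClosestEnemyDistance, which it never updates.
; The tower damages that target, sets dead troops or workers to a new state, destroys them after a delay and retraces; finding no valid target among hits clears the timer.
; Selection events drive the decal and HUD unit widget.
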(event `self.ReceiveBeginPlay`
  (`|ExecutionSequence`
    (:`then_0`
      (bind _returnvalue (`|CreateWidget` "/Game/Licenta/Core/UI/Menus/Unit_Widget/WBP_Unit_Selection_Area.WBP_Unit_Selection_Area_C"))
      (bind _output_get (set `self.UnitSelectedWidget` _returnvalue))
      (set `/Game/Licenta/Core/UI/Menus/Unit_Widget/WBP_Unit_Selection_Area.UnitReference` self _output_get)
      (`Image.SetBrushFromTexture` (`/Game/Licenta/Core/UI/Menus/Unit_Widget/WBP_Unit_Selection_Area.UnitImage` _returnvalue) (`/Game/Licenta/Core/Buildings/BP_BuildingComponent.2D Image` (`self.BP_BuildingComponent`)) false))
    (:`then_1`
      (bind _returnvalue_2 (`KismetSystemLibrary.K2_SetTimerDelegate` (delegate `TraceEnemies`) 3.0 true))
      (set `self.TimeHandle` _returnvalue_2))))

(event `TraceEnemies`
  (bind _returnvalue (`self.K2_GetActorLocation`))
  (bind _targetenemy (`self.TargetEnemy`))
  (bind _returnvalue_2 (`self.GetComponentByClass` _targetenemy "/Game/Licenta/Core/Players/BP_UNIT_SOLDIER.BP_UNIT_SOLDIER_C"))
  (bind (_outhits _returnvalue_3) (`KismetSystemLibrary.SphereTraceMultiForObjects` :`Start` _returnvalue :`End` (+ _returnvalue (0.0 0.0 1.0)) :`Radius` 2000.0 :`ObjectTypes` (`|MakeArray` "ObjectTypeQuery3" :!type "EObjectTypeQuery Enum") :`DrawTime` 1.0 :!label _label))
  (if _returnvalue_3
    (bind _output_get (set `self.TargetEnemy` (`self.GetClosestEnemy` _outhits)))
    (`/Engine/EditorBlueprintResources/StandardMacros.IsValid` _output_get
      (:`Is Valid`
        (`SkeletalMeshComponent.PlayAnimation` (`self.Soldier`) "/Game/Licenta/Core/Players/Soldier/Gunplay__2_.Gunplay__2_" true)
        (`GameplayStatics.ApplyDamage` (`self.TargetEnemy`) (`self.DamageToApply`))
        (`/Engine/EditorBlueprintResources/StandardMacros.IsValid` _targetenemy
          (:`Is Valid`
            (if (`KismetSystemLibrary.IsValid` _returnvalue_2)
              (if (<= (`/Game/Licenta/Core/Players/BP_UNIT_SOLDIER.Health` _returnvalue_2) 0.0)
                (`SkeletalMeshComponent.PlayAnimation` (`self.Soldier`) "/Game/Licenta/Core/Players/Soldier/Rifle_Idle__1_.Rifle_Idle__1_" true)
                (switch `/Game/Licenta/Core/Players/E_PlayerType` (`/Game/Licenta/Core/Players/BP_UNIT_SOLDIER.PlayerType` _returnvalue_2)
                  (:`NewEnumerator1`
                    (`/Game/Licenta/Core/Players/BP_UNIT_SOLDIER.HandleTroopNewUnitState` _returnvalue_2 "NewEnumerator4"))
                  (:`NewEnumerator2`
                    (`/Game/Licenta/Core/Players/BP_UNIT_SOLDIER.HandleWorkerNewUnitState` _returnvalue_2 "NewEnumerator4")))
                (`KismetSystemLibrary.Delay` 3.0)
                (`self.K2_DestroyActor` (`self.TargetEnemy`))
                (goto _label))))))
      (:`Is Not Valid`
        (`self.StopAttack`)))))

(event `StopAttack`
  (`SkeletalMeshComponent.PlayAnimation` (`self.Soldier`) "/Game/Licenta/Core/Players/Soldier/Rifle_Idle__1_.Rifle_Idle__1_" true)
  (`KismetSystemLibrary.K2_ClearAndInvalidateTimerHandle` (`self.TimeHandle`)))

(event `/Game/Licenta/Core/Buildings/BPI_SelectionEvents.SelectThis`
  (`/Game/Licenta/Core/Players/BP_SelectionComponent.ShowSelectionDecal` (`self.BP_SelectionComponent`))
  (message `/Game/Licenta/Core/Buildings/BPI_SelectionEvents.AddUnitToSelectedUnitsArea` (`GameplayStatics.GetPlayerController` 0) (`self.UnitSelectedWidget`)))

(event `/Game/Licenta/Core/Buildings/BPI_SelectionEvents.DeselectThis`
  (`/Game/Licenta/Core/Players/BP_SelectionComponent.HideSelectionDecal` (`self.BP_SelectionComponent`))
  (`Widget.RemoveFromParent` (`self.UnitSelectedWidget`)))

(event `/Game/Licenta/Core/Buildings/BPI_SelectionEvents.HighlightUnit`
  (`DecalComponent.SetDecalMaterial` (`/Game/Licenta/Core/Players/BP_SelectionComponent.DecalComponentRef` (`self.BP_SelectionComponent`)) "/Game/Licenta/Core/Players/M_HightlightIndicator.M_HightlightIndicator"))

(event `/Game/Licenta/Core/Buildings/BPI_SelectionEvents.UnhighlightUnit`
  (`DecalComponent.SetDecalMaterial` (`/Game/Licenta/Core/Players/BP_SelectionComponent.DecalComponentRef` (`self.BP_SelectionComponent`)) "/Game/Licenta/Core/Players/MI_SelectionIndicator.MI_SelectionIndicator"))

(fn `GetClosestEnemy`
  (params (EnemyArray :type "Array of HitResult Structure"))
  (returns (ClosestEnemyRef :type "Actor Object Reference"))
  (locals (ClosestEnemyDistance :type "Float (double-precision)" :default 5e+18) (ClosestEnemy :type "Actor Object Reference"))
  (for _array_element EnemyArray
    (bind (_bblockinghit _binitialoverlap _time _distance _location _impactpoint _normal _impactnormal _physmat _hitactor) (`GameplayStatics.BreakHitResult` _array_element))
    (if (`|EnumEquality` (`/Game/Licenta/Core/Players/BP_UNIT_SOLDIER.TeamAttitude` (`self.GetComponentByClass` _hitactor "/Game/Licenta/Core/Players/BP_UNIT_SOLDIER.BP_UNIT_SOLDIER_C")) "Hostile")
      (if (< (`self.GetDistanceTo` _hitactor self) (`local.ClosestEnemyDistance`))
        (set `local.ClosestEnemy` _hitactor))))
  (return (`local.ClosestEnemy`)))

(fn `UserConstructionScript`
  (`parent.UserConstructionScript`))