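; BP_Building is a building actor for an RTS game that the player can select by clicking.
; A click on a building with Friendly team attitude registers it with the RTS player controller as a selected actor and shows the selection component's decal.
; The building component supplies the team attitude, exposed through a getter, and its destroyed event destroys the actor.
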(event `self.ReceiveActorOnClicked`
  (params (ButtonPressed :type "Key Structure"))
  (`self.BuildingClicked`))

(event `BuildingClicked`
  (if (`|EnumEquality` (`/Game/Licenta/Core/Buildings/BP_BuildingComponent.TeamAttitude` (`self.BP_BuildingComponent`)) "Friendly")
    (`|ExecutionSequence`
      (:`then_0`
        (bind _aspc_rts_game (cast `/Game/Licenta/Core/Players/PC_RTS_GAME` (`GameplayStatics.GetPlayerController` 0)))
        (`/Game/Licenta/Core/Players/PC_RTS_GAME.AddActorSelected` _aspc_rts_game self))
      (:`then_1`
        (`/Game/Licenta/Core/Players/BP_SelectionComponent.ShowSelectionDecal` (`self.BP_SelectionComponent`))))))

(event `self.BP_BuildingComponent.OnBuildingDestroyed`
  (params (TeamAttitude :type "ETeamAttitude Enum" :default "Friendly"))
  (`self.K2_DestroyActor`))

(fn `GetTeamAttitude`
  (returns (TeamAttitude :type "ETeamAttitude Enum"))
  (return (`/Game/Licenta/Core/Buildings/BP_BuildingComponent.TeamAttitude` (`self.BP_BuildingComponent`))))

(fn `UserConstructionScript`)