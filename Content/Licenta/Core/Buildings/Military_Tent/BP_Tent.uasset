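; Military tent building for an RTS that shows a selection decal and UI, with buttons to produce two unit types.
; A looping timer processes the unit queue, tracks progress and spawns finished units at random navigable points within its sphere radius.
; Production time comes from the soldier component on an already-placed actor of the queued class; without one, the queue stalls with a debug print.
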(event `/Game/Licenta/Core/Buildings/BPI_SelectionEvents.SelectThis`
  (`/Game/Licenta/Core/Players/BP_SelectionComponent.ShowSelectionDecal` (`self.BP_SelectionComponent`))
  (`UserWidget.AddToViewport` (`self.BuildingSelectedWidget`) 0))

(event `/Game/Licenta/Core/Buildings/BPI_SelectionEvents.DeselectThis`
  (`/Game/Licenta/Core/Players/BP_SelectionComponent.HideSelectionDecal` (`self.BP_SelectionComponent`))
  (`Widget.RemoveFromParent` (`self.BuildingSelectedWidget`)))

(event `self.ReceiveBeginPlay`
  (`|ExecutionSequence`
    (:`then_0`
      (bind _returnvalue (`|CreateWidget` "/Game/Licenta/Core/UI/Menus/Unit_Widget/Produce_Unit1_Widget.Produce_Unit1_Widget_C"))
      (`KismetArrayLibrary.Array_AddUnique` (`self.ActionBoxButtons`) _returnvalue)
      (set `/Game/Licenta/Core/UI/Menus/Unit_Widget/Produce_Unit1_Widget.BuildingReference` self _returnvalue))
    (:`then_1`
      (bind _returnvalue_2 (`|CreateWidget` "/Game/Licenta/Core/UI/Menus/Unit_Widget/Produce_Unit2_Widget.Produce_Unit2_Widget_C"))
      (`KismetArrayLibrary.Array_AddUnique` (`self.ActionBoxButtons`) _returnvalue_2)
      (set `/Game/Licenta/Core/UI/Menus/Unit_Widget/Produce_Unit2_Widget.BuildingReference` self _returnvalue_2))
    (:`then_2`
      (bind _returnvalue_3 (`|CreateWidget` "/Game/Licenta/Core/UI/Menus/Unit_Widget/WBP_Tent_Selected.WBP_Tent_Selected_C"))
      (bind _output_get (set `self.BuildingSelectedWidget` _returnvalue_3))
      (set `/Game/Licenta/Core/UI/Menus/Unit_Widget/WBP_Tent_Selected.BuildingReference` self _output_get)
      (for _array_element (`self.ActionBoxButtons`)
        (`WrapBox.AddChildToWrapBox` (`/Game/Licenta/Core/UI/Menus/Unit_Widget/WBP_Tent_Selected.ActionBox` (`self.BuildingSelectedWidget`)) _array_element)))
    (:`then_3`
      (`KismetSystemLibrary.K2_SetTimerDelegate` (delegate `ProcessProductionQueue`) (`self.ProductionTimerGranuality`) true))))

(event `AddUnitToQueue`
  (params (Unit :type "Actor Class Reference"))
  (`KismetArrayLibrary.Array_Add` (`self.UnitProductionQueue`) Unit))

(event `ProcessProductionQueue`
  (if (`/Game/Licenta/Core/Buildings/BP_BuildingComponent.isProducingItem` (`self.BP_BuildingComponent`))
    (bind _output_get (set `self.ProductionTimeSpend` (+ (`self.ProductionTimeSpend`) (`self.ProductionTimerGranuality`))))
    (bind _output_get_2 (set `self.ProductionProgress` (/ _output_get (`self.ProductionTimeNeeded`))))
    (if (>= _output_get_2 1.0)
      (bind _randomlocation (`NavigationSystemV1.K2_GetRandomLocationInNavigableRadius` (`self.K2_GetActorLocation`) (`SphereComponent.GetScaledSphereRadius` (`self.Sphere`)) null null))
      (`|SpawnActorFromClass` (`self.UnitBeingProduce`) (`KismetMathLibrary.MakeTransform` (+ _randomlocation (0.0 0.0 100.0))) "AlwaysSpawn" "OverrideRootScale" null null)
      (set `self.ProductionProgress` 0.0)
      (set `self.ProductionTimeSpend` 0.0)
      (set `self.UnitBeingProduce` null)
      (set `/Game/Licenta/Core/Buildings/BP_BuildingComponent.isProducingItem` false (`self.BP_BuildingComponent`)))
    (elif (> (`KismetArrayLibrary.Array_Length` (`self.UnitProductionQueue`)) 0)
      (bind _output_get_3 (set `self.UnitBeingProduce` (`|GetArrayItem` (`self.UnitProductionQueue`))))
      (bind _returnvalue (`GameplayStatics.GetActorOfClass` _output_get_3))
      (bind _returnvalue_2 (`self.GetComponentByClass` _returnvalue "/Game/Licenta/Core/Players/BP_UNIT_SOLDIER.BP_UNIT_SOLDIER_C"))
      (`/Engine/EditorBlueprintResources/StandardMacros.IsValid` _returnvalue_2
        (:`Is Valid`
          (set `self.ProductionTimeNeeded` (`/Game/Licenta/Core/Players/BP_UNIT_SOLDIER.ProductionTime` _returnvalue_2))
          (`KismetArrayLibrary.Array_Remove` (`self.UnitProductionQueue`))
          (set `/Game/Licenta/Core/Buildings/BP_BuildingComponent.isProducingItem` true (`self.BP_BuildingComponent`)))
        (:`Is Not Valid`
          (`KismetSystemLibrary.PrintString` "NO IDEA"))))))

(event `/Game/Licenta/Core/Players/BPI_TOOL_TIPS.SetTooltip`
  (params (TooltipWidget :type "UserWidget Object Reference"))
  (bind _tooltipbox (`/Game/Licenta/Core/UI/Menus/Unit_Widget/WBP_Tent_Selected.TooltipBox` (`self.BuildingSelectedWidget`)))
  ;[1 1 1] Detalis troops
  (`PanelWidget.ClearChildren` _tooltipbox)
  (`/Engine/EditorBlueprintResources/StandardMacros.IsValid` TooltipWidget
    (:`Is Valid`
      (`HorizontalBox.AddChildToHorizontalBox` _tooltipbox TooltipWidget))))

(fn `UserConstructionScript`
  (`parent.UserConstructionScript`))