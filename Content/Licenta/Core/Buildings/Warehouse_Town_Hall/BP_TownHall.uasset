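; Town hall building for an RTS that produces tents and towers, and leaves the game mode's friendly list when destroyed.
; BeginPlay builds its selection panel with two production buttons, shown with a decal on selection.
; A looping timer processes queued buildings one at a time, then calls the matching button widget to create the finished one.
; Production time comes from a world instance found by GetActorOfClass, so one must already exist.
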(event `self.BP_BuildingComponent.OnBuildingDestroyed`
  (params (TeamAttitude :type "ETeamAttitude Enum" :default "Friendly"))
  (bind _asgm_rts_game (cast `/Game/Licenta/Core/Framework/GM_RTS_GAME` (`GameplayStatics.GetGameMode`)))
  (`KismetArrayLibrary.Array_RemoveItem` (`/Game/Licenta/Core/Framework/GM_RTS_GAME.FriendlyTownHalls` _asgm_rts_game) self))

(event `/Game/Licenta/Core/Buildings/BPI_SelectionEvents.SelectThis`
  (`/Game/Licenta/Core/Players/BP_SelectionComponent.ShowSelectionDecal` (`self.BP_SelectionComponent`))
  (`UserWidget.AddToViewport` (`self.BuildingSelectedWidget`) 0))

(event `/Game/Licenta/Core/Buildings/BPI_SelectionEvents.DeselectThis`
  (`/Game/Licenta/Core/Players/BP_SelectionComponent.HideSelectionDecal` (`self.BP_SelectionComponent`))
  (`Widget.RemoveFromParent` (`self.BuildingSelectedWidget`)))

(event `self.ReceiveBeginPlay`
  (`|ExecutionSequence`
    (:`then_0`
      (bind _returnvalue (`|CreateWidget` "/Game/Licenta/Core/UI/Menus/Building_Widget/Produce_Building1_Widget.Produce_Building1_Widget_C"))
      (`KismetArrayLibrary.Array_AddUnique` (`self.ActionBoxImages`) _returnvalue)
      (set `/Game/Licenta/Core/UI/Menus/Building_Widget/Produce_Building1_Widget.BuildingReference` self _returnvalue))
    (:`then_1`
      (bind _returnvalue_2 (`|CreateWidget` "/Game/Licenta/Core/UI/Menus/Building_Widget/Produce_Building2_Widget.Produce_Building2_Widget_C"))
      (`KismetArrayLibrary.Array_AddUnique` (`self.ActionBoxImages`) _returnvalue_2)
      (set `/Game/Licenta/Core/UI/Menus/Building_Widget/Produce_Building2_Widget.BuildingReference` self _returnvalue_2))
    (:`then_2`
      (bind _returnvalue_3 (`|CreateWidget` "/Game/Licenta/Core/UI/Menus/Building_Widget/WBP_Building_Selected.WBP_Building_Selected_C"))
      (bind _output_get (set `self.BuildingSelectedWidget` _returnvalue_3))
      (set `/Game/Licenta/Core/UI/Menus/Building_Widget/WBP_Building_Selected.BuildingReference` self _output_get)
      (for _array_element (`self.ActionBoxImages`)
        (`WrapBox.AddChildToWrapBox` (`/Game/Licenta/Core/UI/Menus/Building_Widget/WBP_Building_Selected.ActionBox` (`self.BuildingSelectedWidget`)) _array_element)))
    (:`then_3`
      (`KismetSystemLibrary.K2_SetTimerDelegate` (delegate `ProcessProductionQueue`) (`self.ProductionTimerGranuality`) true))))

(event `AddBuildingToQueue`
  (params (Unit :type "Actor Class Reference"))
  (`KismetArrayLibrary.Array_Add` (`self.BuildingProductionQueue`) Unit))

(event `ProcessProductionQueue`
  (if (`/Game/Licenta/Core/Buildings/BP_BuildingComponent.isProducingItem` (`self.BP_BuildingComponent`))
    (bind _output_get (set `self.ProductionTimeSpend` (+ (`self.ProductionTimeSpend`) (`self.ProductionTimerGranuality`))))
    (bind _output_get_2 (set `self.ProductionProgress` (/ _output_get (`self.ProductionTimeNeeded`))))
    (if (>= _output_get_2 1.0)
      (set `self.ProductionProgress` 0.0)
      (set `self.ProductionTimeSpend` 0.0)
      (set `/Game/Licenta/Core/Buildings/BP_BuildingComponent.isProducingItem` false (`self.BP_BuildingComponent`))
      (if (== (`self.BuildingBeingProduce`) "/Game/Licenta/Core/Buildings/Military_Tent/BP_Tent.BP_Tent_C")
        (`/Game/Licenta/Core/UI/Menus/Building_Widget/Produce_Building1_Widget.CreateTent` (stale `self.ReceiveBeginPlay` _returnvalue))
        (else
          (`/Game/Licenta/Core/UI/Menus/Building_Widget/Produce_Building2_Widget.CreateTower` (stale `self.ReceiveBeginPlay` _returnvalue_2))))
      (set `self.BuildingBeingProduce` null))
    (elif (> (`KismetArrayLibrary.Array_Length` (`self.BuildingProductionQueue`)) 0)
      (bind _output_get_3 (set `self.BuildingBeingProduce` (`|GetArrayItem` (`self.BuildingProductionQueue`))))
      (bind _returnvalue (`GameplayStatics.GetActorOfClass` _output_get_3))
      (bind _returnvalue_2 (`self.GetComponentByClass` _returnvalue "/Game/Licenta/Core/Buildings/BP_BuildingComponent.BP_BuildingComponent_C"))
      (`/Engine/EditorBlueprintResources/StandardMacros.IsValid` _returnvalue_2
        (:`Is Valid`
          (set `self.ProductionTimeNeeded` (`/Game/Licenta/Core/Buildings/BP_BuildingComponent.ProductionTime` _returnvalue_2))
          (`KismetArrayLibrary.Array_Remove` (`self.BuildingProductionQueue`))
          (set `/Game/Licenta/Core/Buildings/BP_BuildingComponent.isProducingItem` true (`self.BP_BuildingComponent`)))
        (:`Is Not Valid`
          (`KismetSystemLibrary.PrintString` "NO IDEA"))))))

(event `/Game/Licenta/Core/Players/BPI_TOOL_TIPS.SetTooltip`
  (params (TooltipWidget :type "UserWidget Object Reference"))
  (bind _tooltipbox (`/Game/Licenta/Core/UI/Menus/Building_Widget/WBP_Building_Selected.TooltipBox` (`self.BuildingSelectedWidget`)))
  ;[1 1 1] Detalis troops
  (`PanelWidget.ClearChildren` _tooltipbox)
  (`/Engine/EditorBlueprintResources/StandardMacros.IsValid` TooltipWidget
    (:`Is Valid`
      (`HorizontalBox.AddChildToHorizontalBox` _tooltipbox TooltipWidget))))

(fn `UserConstructionScript`
  (`parent.UserConstructionScript`))