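; RTS game mode that decides the match outcome from town hall destruction.
; On BeginPlay it caches enemy and friendly town halls and binds to each building component's destroyed event.
; Any one hall falling with matching Hostile or Friendly attitude shows the winner or loser screen.
; Both town hall getters search for the "Player" tag, but index the hall array by that tag's position, not the matching hall's.
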(event `self.ReceiveBeginPlay`
  (`|ExecutionSequence`
    (:`then_0`
      (bind _outactors (`GameplayStatics.GetAllActorsOfClass` "/Game/Licenta/Core/Players/Enemies/Enemy_Town_Hall/BP_Enemy_TownHall.BP_Enemy_TownHall_C"))
      (bind _output_get (set `self.EnemyTownHalls` _outactors))
      (for _array_element _output_get
        (add `/Game/Licenta/Core/Buildings/BP_BuildingComponent.OnBuildingDestroyed` (`self.GetComponentByClass` _array_element "/Game/Licenta/Core/Buildings/BP_BuildingComponent.BP_BuildingComponent_C") (delegate `OnEnemyTownHallDestroyed`))))
    (:`then_1`
      (bind _outactors_2 (`GameplayStatics.GetAllActorsOfClass` "/Game/Licenta/Core/Buildings/Warehouse_Town_Hall/BP_TownHall.BP_TownHall_C"))
      (bind _output_get_2 (set `self.FriendlyTownHalls` _outactors_2))
      (for _array_element_2 _output_get_2
        (add `/Game/Licenta/Core/Buildings/BP_BuildingComponent.OnBuildingDestroyed` (`self.GetComponentByClass` _array_element_2 "/Game/Licenta/Core/Buildings/BP_BuildingComponent.BP_BuildingComponent_C") (delegate `OnFriendlyTownHallDestroyed`))))))

(event `OnEnemyTownHallDestroyed`
  (params (TeamAttitude :type "ETeamAttitude Enum" :default "Friendly"))
  (if (`|EnumEquality` TeamAttitude "Hostile")
    (`self.WinThisGame`)))

(event `OnFriendlyTownHallDestroyed`
  (params (TeamAttitude :type "ETeamAttitude Enum" :default "Friendly"))
  (if (`|EnumEquality` TeamAttitude "Friendly")
    (`self.LoseThisGame`)))

(event `LoseThisGame`
  (bind _returnvalue (`|CreateWidget` "/Game/Licenta/Core/UI/Menus/WBP_LoserScreen.WBP_LoserScreen_C"))
  (`UserWidget.AddToViewport` _returnvalue 0))

(event `WinThisGame`
  (bind _returnvalue (`|CreateWidget` "/Game/Licenta/Core/UI/Menus/WBP_Winner_Screen.WBP_Winner_Screen_C"))
  (`UserWidget.AddToViewport` _returnvalue 0))

(fn `GetEnemyTownHall`
  (returns (EnemyTownHall :type "Actor Object Reference"))
  (locals (FoundIndex :type Integer) (FoundTownHall :type Integer))
  (bind _enemytownhalls (`self.EnemyTownHalls`))
  (for _array_element _enemytownhalls
    (bind _returnvalue (`KismetArrayLibrary.Array_Find` (`Actor.Tags` _array_element) "Player"))
    (if (>= _returnvalue 0)
      (set `local.FoundIndex` _returnvalue)
      (break)))
  (return (`|GetArrayItem` _enemytownhalls (`local.FoundIndex`))))

(fn `GetPlayerTownHall`
  (returns (PlayerTownHall :type "Actor Object Reference"))
  (locals (FoundIndex :type Integer))
  (for _array_element (`self.FriendlyTownHalls`)
    (bind _returnvalue (`KismetArrayLibrary.Array_Find` (`Actor.Tags` _array_element) "Player"))
    (if (>= _returnvalue 0)
      (set `local.FoundIndex` _returnvalue)
      (break)))
  (return (`|GetArrayItem` (`self.FriendlyTownHalls`) (`local.FoundIndex`))))

(fn `UserConstructionScript`)