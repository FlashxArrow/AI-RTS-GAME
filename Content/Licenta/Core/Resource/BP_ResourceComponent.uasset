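; BP_ResourceComponent makes its owner a gatherable resource with a limited number of uses.
; GiveResources decrements TimesItCanBeMined, fires OnResourceGathered, then returns the resource type and amount to give.
; It also fires the exhausted event when CanThisResourceBeMinded reports no uses left.
; GiveResources does not check remaining uses before paying out.
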(fn `CanThisResourceBeMinded`
  (returns (ReturnValue :type Boolean))
  (return (> (`self.TimesItCanBeMined`) 0)))

(fn `Give Resources`
  (returns (TypeOfResource :type "/Game/Licenta/Core/Resource/E_ResourceType Enum") (NumberOfResourcesToGive :type Integer))
  (set `self.TimesItCanBeMined` (- (`self.TimesItCanBeMined`) 1))
  (`self.OnResourceGathered`)
  (`|ExecutionSequence`
    (:`then_0`
      (if (not (`self.CanThisResourceBeMinded`))
        (`self.OneResourceExhausted`)))
    (:`then_1`
      (return (`self.TypeOfResource`) (`self.NumberOfResourcesToGive`)))))