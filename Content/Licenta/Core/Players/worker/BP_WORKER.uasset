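; RTS worker unit that moves on command, gathers resources and deposits them at the player's town hall.
; AI MoveTo drives a gather loop: mine after a retriggerable delay, deliver to the player controller, then repeat while the resource remains mineable.
; State changes go through the BP_UNIT_SOLDIER component, whose event selects the matching animation.
; Selection and highlighting use decals, plus a portrait widget created on BeginPlay.
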(event `self.BP_UNIT_SOLDIER.OnEnterWorkerState`
  (params (NewState :type "/Game/Licenta/Core/Players/worker/E_WorkerUnitStates Enum" :default "NewEnumerator0"))
  (`SkeletalMeshComponent.PlayAnimation` (`self.Mesh`) (select `/Game/Licenta/Core/Players/worker/E_WorkerUnitStates` NewState :`NewEnumerator1` "/Game/Licenta/Core/Players/worker/A_idle.A_idle" :`NewEnumerator2` "/Game/Licenta/Core/Players/worker/A_Walk.A_Walk" :`NewEnumerator3` "/Game/Licenta/Core/Players/worker/A_mining.A_mining" :`NewEnumerator4` "/Game/Licenta/Core/Players/worker/A_death.A_death" :!type "AnimationAsset Object Reference") (`|EnumInequality` NewState "NewEnumerator4")))

(event `self.ReceiveBeginPlay`
  (bind _returnvalue (`|CreateWidget` "/Game/Licenta/Core/UI/Menus/Unit_Widget/WBP_Unit_Selection_Area.WBP_Unit_Selection_Area_C"))
  (bind _output_get (set `self.UnitSelectedWidget ` _returnvalue))
  (set `/Game/Licenta/Core/UI/Menus/Unit_Widget/WBP_Unit_Selection_Area.UnitReference` self _output_get)
  (`Image.SetBrushFromTexture` (`/Game/Licenta/Core/UI/Menus/Unit_Widget/WBP_Unit_Selection_Area.UnitImage` _returnvalue) (`/Game/Licenta/Core/Players/BP_UNIT_SOLDIER.2D_Image` (`self.BP_UNIT_SOLDIER`)) false))

(event `/Game/Licenta/Core/Players/BPI_UNIT_ACTION.MoveToThisLocation`
  (params (GoalLocation :type "Vector Structure"))
  (`/Game/Licenta/Core/Players/BP_UNIT_SOLDIER.HandleWorkerNewUnitState` (`self.BP_UNIT_SOLDIER`) "NewEnumerator2")
  (bind _movementresult (`|AIMoveTo` self GoalLocation null 50.0)
    (:`OnSuccess`
      _)
    (:`OnFail`
      (switch `EPathFollowingResult` _movementresult
        (:`Blocked`
          _)
        (:`OffPath`
          _)
        (:`Invalid`
          _))))
  (`/Game/Licenta/Core/Players/BP_UNIT_SOLDIER.HandleWorkerNewUnitState` (`self.BP_UNIT_SOLDIER`) "NewEnumerator1"))

(event `/Game/Licenta/Core/Players/BPI_UNIT_ACTION.GatherThisResource`
  (params (ResourceRef :type "Actor Object Reference"))
  (bind _returnvalue (`self.GetComponentByClass` ResourceRef "/Game/Licenta/Core/Resource/BP_ResourceComponent.BP_ResourceComponent_C"))
  (bind (_returnvalue_roll _returnvalue_pitch _returnvalue_yaw) (`KismetMathLibrary.BreakRotator` (`KismetMathLibrary.FindLookAtRotation` (`self.K2_GetActorLocation`) (`self.K2_GetActorLocation` ResourceRef))))
  ;[1 1 1] Move towards the resource and look towards it
  (`/Game/Licenta/Core/Players/BP_UNIT_SOLDIER.HandleWorkerNewUnitState` (`self.BP_UNIT_SOLDIER`) "NewEnumerator2")
  (`|AIMoveTo` self (0.0 0.0 0.0) ResourceRef 200.0
    (:`OnSuccess`
      (`self.K2_SetActorRotation` (`KismetMathLibrary.MakeRotator` 0.0 0.0 _returnvalue_yaw))
      ;[1 1 1] Mining resource
      (`/Engine/EditorBlueprintResources/StandardMacros.IsValid` _returnvalue
        (:`Is Valid`
          (if (and (`/Game/Licenta/Core/Resource/BP_ResourceComponent.CanThisResourceBeMinded` _returnvalue) (`|EnumInequality` (`self.ResourceBeingCarried`) (`/Game/Licenta/Core/Resource/BP_ResourceComponent.TypeOfResource` _returnvalue)))
            (`/Game/Licenta/Core/Players/BP_UNIT_SOLDIER.HandleWorkerNewUnitState` (`self.BP_UNIT_SOLDIER`) "NewEnumerator3")
            (set `self.AmountOfResources` 0)
            (`KismetSystemLibrary.RetriggerableDelay` (`/Game/Licenta/Core/Resource/BP_ResourceComponent.TimesItTakesToGatherInSeconds` _returnvalue))
            ;[1 1 1] Getting resource
            (if (`|EnumEquality` (`/Game/Licenta/Core/Players/BP_UNIT_SOLDIER.WorkerUnitState` (`self.BP_UNIT_SOLDIER`)) "NewEnumerator3")
              (bind (_typeofresource _numberofresourcestogive) (`/Game/Licenta/Core/Resource/BP_ResourceComponent.Give Resources` _returnvalue))
              (set `self.ResourceBeingCarried` _typeofresource)
              (set `self.AmountOfResources` _numberofresourcestogive)
              (`self.GoToTownHallAndDepositResources` ResourceRef)
              (else
                (`/Game/Licenta/Core/Players/BP_UNIT_SOLDIER.HandleWorkerNewUnitState` (`self.BP_UNIT_SOLDIER`) "NewEnumerator1")))
            (elif (and (`|EnumEquality` (`self.ResourceBeingCarried`) (`/Game/Licenta/Core/Resource/BP_ResourceComponent.TypeOfResource` _returnvalue)) (> (`self.AmountOfResources`) 0))
              (`self.GoToTownHallAndDepositResources` ResourceRef)
              (else
                (`/Game/Licenta/Core/Players/BP_UNIT_SOLDIER.HandleWorkerNewUnitState` (`self.BP_UNIT_SOLDIER`) "NewEnumerator1")))))))))

(event `GoToTownHallAndDepositResources`
  (params (ResourceRef :type "Actor Object Reference"))
  (`/Game/Licenta/Core/Players/BP_UNIT_SOLDIER.HandleWorkerNewUnitState` (`self.BP_UNIT_SOLDIER`) "NewEnumerator2")
  (bind _asgm_rts_game (cast `/Game/Licenta/Core/Framework/GM_RTS_GAME` (`GameplayStatics.GetGameMode`)))
  (bind _suitablelocationref (`/Game/Licenta/Core/Buildings/BP_BuildingComponent.GetSuitableLocation` (`self.GetComponentByClass` (`/Game/Licenta/Core/Framework/GM_RTS_GAME.GetPlayerTownHall` _asgm_rts_game) "/Game/Licenta/Core/Buildings/BP_BuildingComponent.BP_BuildingComponent_C")))
  (`/Engine/EditorBlueprintResources/StandardMacros.IsValid` _suitablelocationref
    (:`Is Valid`
      (`|AIMoveTo` self (`SceneComponent.K2_GetComponentLocation` _suitablelocationref) null 1.0 true
        (:`OnSuccess`
          (`/Game/Licenta/Core/Players/BP_UNIT_SOLDIER.HandleWorkerNewUnitState` (`self.BP_UNIT_SOLDIER`) "NewEnumerator1")
          (bind _aspc_rts_game (cast `/Game/Licenta/Core/Players/PC_RTS_GAME` (`GameplayStatics.GetPlayerController` 0)))
          (`/Game/Licenta/Core/Players/PC_RTS_GAME.ReceiveResources` _aspc_rts_game (`self.ResourceBeingCarried`) (`self.AmountOfResources`))
          (set `self.ResourceBeingCarried` "NewEnumerator0")
          (set `self.AmountOfResources` 0)
          (`/Engine/EditorBlueprintResources/StandardMacros.IsValid` ResourceRef
            (:`Is Valid`
              (`self.RepeatTheMiningAction` ResourceRef))))))
    (:`Is Not Valid`
      (`/Game/Licenta/Core/Players/BP_UNIT_SOLDIER.HandleWorkerNewUnitState` (`self.BP_UNIT_SOLDIER`) "NewEnumerator1"))))

(event `RepeatTheMiningAction`
  (params (ResourceRef :type "Actor Object Reference"))
  (if (`/Game/Licenta/Core/Resource/BP_ResourceComponent.CanThisResourceBeMinded` (`self.GetComponentByClass` ResourceRef "/Game/Licenta/Core/Resource/BP_ResourceComponent.BP_ResourceComponent_C"))
    (`/Game/Licenta/Core/Players/BPI_UNIT_ACTION.GatherThisResource` ResourceRef)))

(event `/Game/Licenta/Core/Players/BPI_UNIT_ACTION.InteractWithBuilding`
  (params (BuildingRef :type "Actor Object Reference"))
  (bind _returnvalue (`self.GetComponentByClass` BuildingRef "/Game/Licenta/Core/Buildings/BP_BuildingComponent.BP_BuildingComponent_C"))
  (`/Engine/EditorBlueprintResources/StandardMacros.IsValid` _returnvalue
    (:`Is Valid`
      (if (> (`self.AmountOfResources`) 0)
        (if (`|EnumEquality` (`/Game/Licenta/Core/Buildings/BP_BuildingComponent.TypeOfBuilding` _returnvalue) "NewEnumerator1")
          (`self.GoToTownHallAndDepositResources` null))))))

(event `/Game/Licenta/Core/Buildings/BPI_SelectionEvents.SelectThis`
  (`/Game/Licenta/Core/Players/BP_SelectionComponent.ShowSelectionDecal` (`self.BP_SelectionComponent`))
  (message `/Game/Licenta/Core/Buildings/BPI_SelectionEvents.AddUnitToSelectedUnitsArea` (`GameplayStatics.GetPlayerController` 0) (`self.UnitSelectedWidget `)))

(event `/Game/Licenta/Core/Buildings/BPI_SelectionEvents.DeselectThis`
  (`/Game/Licenta/Core/Players/BP_SelectionComponent.HideSelectionDecal` (`self.BP_SelectionComponent`))
  (`Widget.RemoveFromParent` (`self.UnitSelectedWidget `)))

(event `self.CapsuleComponent.OnClicked`
  (params (TouchedComponent :type "PrimitiveComponent Object Reference") (ButtonPressed :type "Key Structure"))
  (message `/Game/Licenta/Core/Buildings/BPI_SelectionEvents.ClickSelectThisActor` (`GameplayStatics.GetPlayerController` 0) self))

(event `/Game/Licenta/Core/Buildings/BPI_SelectionEvents.HighlightUnit`
  (`DecalComponent.SetDecalMaterial` (`/Game/Licenta/Core/Players/BP_SelectionComponent.DecalComponentRef` (`self.BP_SelectionComponent`)) "/Game/Licenta/Core/Players/M_HightlightIndicator.M_HightlightIndicator"))

(event `/Game/Licenta/Core/Buildings/BPI_SelectionEvents.UnhighlightUnit`
  (`DecalComponent.SetDecalMaterial` (`/Game/Licenta/Core/Players/BP_SelectionComponent.DecalComponentRef` (`self.BP_SelectionComponent`)) "/Game/Licenta/Core/Players/MI_SelectionIndicator.MI_SelectionIndicator"))

(fn `GetTeamAttitude`
  (returns (TeamAttitude :type "ETeamAttitude Enum"))
  (return (`/Game/Licenta/Core/Players/BP_UNIT_SOLDIER.TeamAttitude` (`self.BP_UNIT_SOLDIER`))))

(fn `UserConstructionScript`)