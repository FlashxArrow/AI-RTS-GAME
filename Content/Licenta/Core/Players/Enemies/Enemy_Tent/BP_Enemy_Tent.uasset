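; Enemy military tent building that produces units from a queue, requesting two townhall troops through the player controller shortly after BeginPlay.
; AddEnemyUnitToQueue fills the queue, and a looping timer advances production progress, then spawns the finished unit at a random navigable point within the tent's sphere radius.
; Production time comes from the soldier component of an existing world instance of the queued class, so production only starts when one is found.
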(event `self.ReceiveBeginPlay`
  (bind _returnvalue (`GameplayStatics.GetPlayerController` 0))
  (`|ExecutionSequence`
    (:`then_0`
      (`KismetSystemLibrary.Delay` 5.0)
      (message `/Game/Licenta/Core/Buildings/BPI_SelectionEvents.ProduceEnemyUnit` _returnvalue self "/Game/Licenta/Core/Players/Enemies/Enemy_soldier/Attack_TownHall/BP_TROOP_TOWNHALL.BP_TROOP_TOWNHALL_C"))
    (:`then_1`
      (`KismetSystemLibrary.Delay` 5.0)
      (message `/Game/Licenta/Core/Buildings/BPI_SelectionEvents.ProduceEnemyUnit` _returnvalue self "/Game/Licenta/Core/Players/Enemies/Enemy_soldier/Attack_TownHall/BP_TROOP_TOWNHALL.BP_TROOP_TOWNHALL_C"))
    (:`then_2`
      (`KismetSystemLibrary.K2_SetTimerDelegate` (delegate `ProcessProductionQueue`) (`self.ProductionTimerGranuality`) true))))

(event `AddEnemyUnitToQueue`
  (params (Unit :type "Actor Class Reference (by ref)"))
  (`KismetArrayLibrary.Array_Add` (`self.UnitProductionQueue`) Unit))

(event `ProcessProductionQueue`
  (if (`/Game/Licenta/Core/Buildings/BP_BuildingComponent.isProducingItem` (`self.BP_BuildingComponent`))
    (bind _output_get (set `self.ProductionTimeSpend` (+ (`self.ProductionTimeSpend`) (`self.ProductionTimerGranuality`))))
    (bind _output_get_2 (set `self.ProductionProgress` (/ _output_get (`self.ProductionTimeNeeded`))))
    (if (>= _output_get_2 1.0)
      (bind _randomlocation (`NavigationSystemV1.K2_GetRandomLocationInNavigableRadius` (`self.K2_GetActorLocation`) (`SphereComponent.GetScaledSphereRadius` (`self.Sphere`)) null null))
      (`|SpawnActorFromClass` (`self.UnitBeingProduce`) (`KismetMathLibrary.MakeTransform` _randomlocation) "AlwaysSpawn" "OverrideRootScale" null null)
      (set `self.ProductionProgress` 0.0)
      (set `self.ProductionTimeSpend` 0.0)
      (set `self.UnitBeingProduce` null)
      (set `/Game/Licenta/Core/Buildings/BP_BuildingComponent.isProducingItem` false (`self.BP_BuildingComponent`)))
    (elif (> (`KismetArrayLibrary.Array_Length` (`self.UnitProductionQueue`)) 0)
      (bind _output_get_3 (set `self.UnitBeingProduce` (`|GetArrayItem` (`self.UnitProductionQueue`))))
      (bind _returnvalue (`GameplayStatics.GetActorOfClass` _output_get_3))
      (bind _returnvalue_2 (`self.GetComponentByClass` _returnvalue "/Game/Licenta/Core/Players/BP_UNIT_SOLDIER.BP_UNIT_SOLDIER_C"))
      (`/Engine/EditorBlueprintResources/StandardMacros.IsValid` _returnvalue_2
        (:`Is Valid`
          (set `self.ProductionTimeNeeded` (`/Game/Licenta/Core/Players/BP_UNIT_SOLDIER.ProductionTime` _returnvalue_2))
          (`KismetArrayLibrary.Array_Remove` (`self.UnitProductionQueue`))
          (set `/Game/Licenta/Core/Buildings/BP_BuildingComponent.isProducingItem` true (`self.BP_BuildingComponent`)))))))

(fn `UserConstructionScript`
  (`parent.UserConstructionScript`))