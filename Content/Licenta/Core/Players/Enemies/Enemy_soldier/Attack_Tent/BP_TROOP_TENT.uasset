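; Selectable RTS troop unit that moves and attacks units or buildings, with stats and animation state held in its BP_UNIT_SOLDIER component.
; Selection toggles a decal and adds a portrait widget through the player controller.
; Attack orders use AIMoveTo, then a looping timer for damage, re-chasing targets beyond the distance recorded when ordered.
; Defeated units play death states and are destroyed after a delay, while building-destruction logic is left unconnected.
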(event `self.ReceiveBeginPlay`
  ;[1 1 1] SelectedWidgetUnit
  (bind _returnvalue (`|CreateWidget` "/Game/Licenta/Core/UI/Menus/Unit_Widget/WBP_Unit_Selection_Area.WBP_Unit_Selection_Area_C"))
  (bind _output_get (set `self.UnitSelectedWidget ` _returnvalue))
  (set `/Game/Licenta/Core/UI/Menus/Unit_Widget/WBP_Unit_Selection_Area.UnitReference` self _output_get)
  (`Image.SetBrushFromTexture` (`/Game/Licenta/Core/UI/Menus/Unit_Widget/WBP_Unit_Selection_Area.UnitImage` _returnvalue) (`/Game/Licenta/Core/Players/BP_UNIT_SOLDIER.2D_Image` (`self.BP_UNIT_SOLDIER`)) false))

(event `self.MoveToThisLocation`
  (params (GoalLocation :type "Vector Structure"))
  (`/Game/Licenta/Core/Players/BP_UNIT_SOLDIER.HandleTroopNewUnitState` (`self.BP_UNIT_SOLDIER`) "NewEnumerator2")
  (bind _movementresult (`|AIMoveTo` self GoalLocation null 50.0)
    (:`OnSuccess`
      _)
    (:`OnFail`
      (switch `EPathFollowingResult` _movementresult
        (:`Blocked`
          _)
        (:`OffPath`
          _)
        (:`Invalid`
          _))))
  (`/Game/Licenta/Core/Players/BP_UNIT_SOLDIER.HandleTroopNewUnitState` (`self.BP_UNIT_SOLDIER`) "NewEnumerator1"))

(event `self.AttackThisActor`
  (params (ActorToAttack :type "Actor Object Reference"))
  (bind _actor_to_attack (`self.Actor to Attack`))
  (bind _actor_to_attack_2 (`self.Actor to Attack`))
  (bind _returnvalue (`self.GetComponentByClass` _actor_to_attack_2 "/Game/Licenta/Core/Buildings/BP_BuildingComponent.BP_BuildingComponent_C"))
  (bind (_returnvalue_roll _returnvalue_pitch _returnvalue_yaw) (`KismetMathLibrary.BreakRotator` (`KismetMathLibrary.FindLookAtRotation` (`self.K2_GetActorLocation`) (`self.K2_GetActorLocation` _actor_to_attack))))
  (set `self.Actor to Attack` ActorToAttack)
  (`/Game/Licenta/Core/Players/BP_UNIT_SOLDIER.HandleTroopNewUnitState` (`self.BP_UNIT_SOLDIER`) "NewEnumerator2")
  (set `self.RangeToAttack` (`KismetMathLibrary.Vector_Distance` (`self.K2_GetActorLocation` _actor_to_attack_2) (`self.K2_GetActorLocation`)))
  (`/Engine/EditorBlueprintResources/StandardMacros.IsValid` _returnvalue
    (:`Is Valid`
      (`|AIMoveTo` self (`SceneComponent.K2_GetComponentLocation` (`/Game/Licenta/Core/Buildings/BP_BuildingComponent.GetSuitableLocation` _returnvalue)) null 200.0 true
        (:`OnSuccess`
          _)))
    (:`Is Not Valid`
      (`|AIMoveTo` self (0.0 0.0 0.0) (`self.Actor to Attack`)
        (:`OnSuccess`
          _))))
  (`/Engine/EditorBlueprintResources/StandardMacros.IsValid` _actor_to_attack
    (:`Is Valid`
      (`self.K2_SetActorRotation` (`KismetMathLibrary.MakeRotator` 0.0 0.0 _returnvalue_yaw))
      (`/Game/Licenta/Core/Players/BP_UNIT_SOLDIER.HandleTroopNewUnitState` (`self.BP_UNIT_SOLDIER`) "NewEnumerator3")
      (bind _returnvalue_2 (`KismetSystemLibrary.K2_SetTimerDelegate` (`|CreateDelegate` :!event `Attack`) 1.0 true))
      (set `self.AttackTimer` _returnvalue_2))
    (:`Is Not Valid`
      (`self.StopAttack`))))

(event `Attack`
  (bind _actor_to_attack (`self.Actor to Attack`))
  (if (>= (`/Game/Licenta/Core/Players/BP_UNIT_SOLDIER.Health` (`self.BP_UNIT_SOLDIER`)) 0.0)
    (`self.Actor to Attack`
      (:`then`
        (if (<= (`KismetMathLibrary.Vector_Distance` (`self.K2_GetActorLocation` (`self.Actor to Attack`)) (`self.K2_GetActorLocation`)) (`self.RangeToAttack`))
          (`GameplayStatics.ApplyDamage` (`self.Actor to Attack`) (`/Game/Licenta/Core/Players/BP_UNIT_SOLDIER.DamageToApply` (`self.BP_UNIT_SOLDIER`)))
          (`self.DefeatedActor`)
          (else
            (`KismetSystemLibrary.K2_ClearAndInvalidateTimerHandle` (`self.AttackTimer`))
            (if (`|EnumEquality` (`/Game/Licenta/Core/Players/BP_UNIT_SOLDIER.TroopUnitState` (`self.BP_UNIT_SOLDIER`)) "NewEnumerator3")
              (`/Engine/EditorBlueprintResources/StandardMacros.IsValid` _actor_to_attack
                (:`Is Valid`
                  (`self.AttackThisActor` _actor_to_attack)))))))
      (:`else`
        (`self.StopAttack`)))))

(event `self.BP_UNIT_SOLDIER.OnEnterTroopState`
  (params (NewState :type "/Game/Licenta/Core/Players/Soldier/E_TroopUnitStates Enum" :default "NewEnumerator0"))
  (`SkeletalMeshComponent.PlayAnimation` (`self.Mesh`) (select `/Game/Licenta/Core/Players/Soldier/E_TroopUnitStates` NewState :`NewEnumerator1` "/Game/Licenta/Core/Players/Soldier/Rifle_Idle__1_.Rifle_Idle__1_" :`NewEnumerator2` "/Game/Licenta/Core/Players/Soldier/Rifle_Walk.Rifle_Walk" :`NewEnumerator3` "/Game/Licenta/Core/Players/Soldier/Gunplay__2_.Gunplay__2_" :`NewEnumerator4` "/Game/Licenta/Core/Players/Soldier/Death.Death" :!type "AnimationAsset Object Reference") (`|EnumInequality` NewState "NewEnumerator4")))

(event `/Game/Licenta/Core/Buildings/BPI_SelectionEvents.SelectThis`
  (`/Game/Licenta/Core/Players/BP_SelectionComponent.ShowSelectionDecal` (`self.BP_SelectionComponent`))
  (message `/Game/Licenta/Core/Buildings/BPI_SelectionEvents.AddUnitToSelectedUnitsArea` (`GameplayStatics.GetPlayerController` 0) (`self.UnitSelectedWidget `)))

(event `/Game/Licenta/Core/Buildings/BPI_SelectionEvents.DeselectThis`
  (`/Game/Licenta/Core/Players/BP_SelectionComponent.HideSelectionDecal` (`self.BP_SelectionComponent`))
  (`Widget.RemoveFromParent` (`self.UnitSelectedWidget `)))

(event `self.CapsuleComponent.OnClicked`
  (params (TouchedComponent :type "PrimitiveComponent Object Reference") (ButtonPressed :type "Key Structure"))
  (if (`|EnumEquality` (`/Game/Licenta/Core/Players/BP_UNIT_SOLDIER.TeamAttitude` (`self.BP_UNIT_SOLDIER`)) "Friendly")
    (message `/Game/Licenta/Core/Buildings/BPI_SelectionEvents.ClickSelectThisActor` (`GameplayStatics.GetPlayerController` 0) self)))

(event `self.DefeatedActor`
  (bind _actor_to_attack (`self.Actor to Attack`))
  (bind _actor_to_attack_2 (`self.Actor to Attack`))
  (bind _returnvalue (`self.GetComponentByClass` _actor_to_attack_2 "/Game/Licenta/Core/Players/BP_UNIT_SOLDIER.BP_UNIT_SOLDIER_C"))
  ;[1 1 1] Deafeted
  (`/Engine/EditorBlueprintResources/StandardMacros.IsValid` _actor_to_attack_2
    (:`Is Valid`
      (if (`KismetSystemLibrary.IsValid` _returnvalue)
        (if (<= (`/Game/Licenta/Core/Players/BP_UNIT_SOLDIER.Health` _returnvalue) 0.0)
          (`self.StopAttack`)
          (switch `/Game/Licenta/Core/Players/E_PlayerType` (`/Game/Licenta/Core/Players/BP_UNIT_SOLDIER.PlayerType` _returnvalue)
            (:`NewEnumerator1`
              (`/Game/Licenta/Core/Players/BP_UNIT_SOLDIER.HandleTroopNewUnitState` _returnvalue "NewEnumerator4"))
            (:`NewEnumerator2`
              (`/Game/Licenta/Core/Players/BP_UNIT_SOLDIER.HandleWorkerNewUnitState` _returnvalue "NewEnumerator4")))
          (`KismetSystemLibrary.Delay` 3.0)
          (`self.K2_DestroyActor` (`self.Actor to Attack`)))
        (else
          (`/Engine/EditorBlueprintResources/StandardMacros.IsValid` _actor_to_attack
            (:`Is Valid`
              (switch `/Game/Licenta/Core/Buildings/E_BuildingTypes` (`/Game/Licenta/Core/Buildings/BP_BuildingComponent.TypeOfBuilding` (`self.GetComponentByClass` _actor_to_attack "/Game/Licenta/Core/Buildings/BP_BuildingComponent.BP_BuildingComponent_C"))
                (:`NewEnumerator0`
                  (`KismetSystemLibrary.PrintString` "done!"))
                (:`NewEnumerator1`
                  (bind _returnvalue_2 (`GameplayStatics.GetActorOfClass` "/Game/Licenta/Core/Buildings/Warehouse_Town_Hall/BP_TownHall.BP_TownHall_C")))
                (:`NewEnumerator2`
                  (bind _returnvalue_3 (`GameplayStatics.GetActorOfClass` "/Game/Licenta/Core/Buildings/Military_Hut/BP_FINAL_HUT.BP_FINAL_HUT_C")))
                (:`NewEnumerator3`
                  (bind _returnvalue_4 (`GameplayStatics.GetActorOfClass` "/Game/Licenta/Core/Buildings/Military_Tent/BP_Tent.BP_Tent_C")))
                (:`NewEnumerator4`
                  (bind _returnvalue_5 (`GameplayStatics.GetActorOfClass` "/Game/Licenta/Core/Buildings/Military_Tower/BP_Tower.BP_Tower_C")))))))))))

(event `/Game/Licenta/Core/Buildings/BPI_SelectionEvents.HighlightUnit`
  (`DecalComponent.SetDecalMaterial` (`/Game/Licenta/Core/Players/BP_SelectionComponent.DecalComponentRef` (`self.BP_SelectionComponent`)) "/Game/Licenta/Core/Players/M_HightlightIndicator.M_HightlightIndicator"))

(event `StopAttack`
  (`/Game/Licenta/Core/Players/BP_UNIT_SOLDIER.HandleTroopNewUnitState` (`self.BP_UNIT_SOLDIER`) "NewEnumerator1")
  (`KismetSystemLibrary.K2_ClearAndInvalidateTimerHandle` (`self.AttackTimer`)))

(event `/Game/Licenta/Core/Buildings/BPI_SelectionEvents.UnhighlightUnit`
  (`DecalComponent.SetDecalMaterial` (`/Game/Licenta/Core/Players/BP_SelectionComponent.DecalComponentRef` (`self.BP_SelectionComponent`)) "/Game/Licenta/Core/Players/MI_SelectionIndicator.MI_SelectionIndicator"))

(fn `GetTeamAttitude`
  (returns (TeamAttitude :type "ETeamAttitude Enum"))
  (return (`/Game/Licenta/Core/Players/BP_UNIT_SOLDIER.TeamAttitude` (`self.BP_UNIT_SOLDIER`))))

(fn `UserConstructionScript`)