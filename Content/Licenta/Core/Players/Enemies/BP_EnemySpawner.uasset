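; Enemy spawner actor that periodically creates BP_ENEMY_TROOP1 troops around its own location.
; BeginPlay starts a looping timer on a configurable interval and stores its handle; SpawnWave picks a small random count for SpawnEnemy.
; SpawnEnemy places each troop at a random navigable point within the scaled radius of its Sphere component.
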(event `self.ReceiveBeginPlay`
  (bind _returnvalue (`KismetSystemLibrary.K2_SetTimerDelegate` (`|CreateDelegate` :!event `SpawnWave`) (`self.SpawnEnemiesXSeconds`) true 0.0 2.0))
  (set `self.SpawnTimer` _returnvalue))

(event `SpawnWave`
  (`self.SpawnEnemy` (`KismetMathLibrary.RandomIntegerInRange` 1 2)))

(event `SpawnEnemy`
  (params (EnemiesToASpawn :type Integer :default 1))
  (for _ (range 1 (+ EnemiesToASpawn 1))
    (bind _randomlocation (`NavigationSystemV1.K2_GetRandomLocationInNavigableRadius` (`self.K2_GetActorLocation`) (`SphereComponent.GetScaledSphereRadius` (`self.Sphere`)) null null))
    (`|SpawnActorFromClass` "/Game/Licenta/Core/Players/Enemies/EnemySoldier/AttackCloseSoldier/BP_ENEMY_TROOP1.BP_ENEMY_TROOP1_C" (`KismetMathLibrary.MakeTransform` _randomlocation) "Undefined" "OverrideRootScale" null null)))

(fn `UserConstructionScript`)