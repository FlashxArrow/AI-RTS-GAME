(event `self.BP_BuildingComponent.OnBuildingDestroyed`
  (params (TeamAttitude :type "ETeamAttitude Enum" :default "Friendly"))
  (bind _asgm_rts_game (cast `/Game/Licenta/Core/Framework/GM_RTS_GAME` (`GameplayStatics.GetGameMode`)))
  (`KismetArrayLibrary.Array_RemoveItem` (`/Game/Licenta/Core/Framework/GM_RTS_GAME.EnemyTownHalls` _asgm_rts_game) self))

(event `self.ReceiveBeginPlay`
  (bind _returnvalue (`GameplayStatics.GetPlayerController` 0))
  (`|ExecutionSequence`
    (:`then_0`
      (`KismetSystemLibrary.Delay` 5.0)
      (message `/Game/Licenta/Core/Buildings/BPI_SelectionEvents.ProduceEnemyBuilding` _returnvalue self "/Game/Licenta/Core/Players/Enemies/Enemy_Tower/BP_Enemy_Tower.BP_Enemy_Tower_C"))
    (:`then_1`
      (`KismetSystemLibrary.Delay` 5.0)
      (message `/Game/Licenta/Core/Buildings/BPI_SelectionEvents.ProduceEnemyBuilding` _returnvalue self "/Game/Licenta/Core/Players/Enemies/Enemy_Tent/BP_Enemy_Tent.BP_Enemy_Tent_C"))
    (:`then_2`
      (`KismetSystemLibrary.K2_SetTimerDelegate` (delegate `ProcessProductionQueue`) (`self.ProductionTimerGranuality`) true))))

(event `AddEnemyBuildingToQueue`
  (params (Unit :type "Actor Class Reference"))
  (`KismetArrayLibrary.Array_Add` (`self.BuildingProductionQueue`) Unit))

(event `ProcessProductionQueue`
  (if (`/Game/Licenta/Core/Buildings/BP_BuildingComponent.isProducingItem` (`self.BP_BuildingComponent`))
    (bind _output_get (set `self.ProductionTimeSpend` (+ (`self.ProductionTimeSpend`) (`self.ProductionTimerGranuality`))))
    (bind _output_get_2 (set `self.ProductionProgress` (/ _output_get (`self.ProductionTimeNeeded`))))
    (if (>= _output_get_2 1.0)
      (set `self.ProductionProgress` 0.0)
      (set `self.ProductionTimeSpend` 0.0)
      (set `/Game/Licenta/Core/Buildings/BP_BuildingComponent.isProducingItem` false (`self.BP_BuildingComponent`))
      (if (== (`self.BuildingBeingProduce`) "/Game/Licenta/Core/Players/Enemies/Enemy_Tent/BP_Enemy_Tent.BP_Enemy_Tent_C")
        (`|SpawnActorFromClass` "/Game/Licenta/Core/Players/Enemies/Enemy_Tent/BP_Enemy_Tent.BP_Enemy_Tent_C" (`KismetMathLibrary.MakeTransform` (1910.0 -16100.0 100.0) (struct :`Yaw` 180.0)) "AlwaysSpawn" "OverrideRootScale" null null)
        (else
          (`|SpawnActorFromClass` "/Game/Licenta/Core/Players/Enemies/Enemy_Tower/BP_Enemy_Tower.BP_Enemy_Tower_C" (`KismetMathLibrary.MakeTransform` (7360.0 -16390.0 70.0) (struct :`Yaw` 180.0)) "AlwaysSpawn" "OverrideRootScale" null null)))
      (set `self.BuildingBeingProduce` null))
    (elif (> (`KismetArrayLibrary.Array_Length` (`self.BuildingProductionQueue`)) 0)
      (bind _output_get_3 (set `self.BuildingBeingProduce` (`|GetArrayItem` (`self.BuildingProductionQueue`))))
      (bind _returnvalue (`GameplayStatics.GetActorOfClass` _output_get_3))
      (bind _returnvalue_2 (`self.GetComponentByClass` _returnvalue "/Game/Licenta/Core/Buildings/BP_BuildingComponent.BP_BuildingComponent_C"))
      (`/Engine/EditorBlueprintResources/StandardMacros.IsValid` _returnvalue_2
        (:`Is Valid`
          (set `self.ProductionTimeNeeded` (`/Game/Licenta/Core/Buildings/BP_BuildingComponent.ProductionTime` _returnvalue_2))
          (`KismetArrayLibrary.Array_Remove` (`self.BuildingProductionQueue`))
          (set `/Game/Licenta/Core/Buildings/BP_BuildingComponent.isProducingItem` true (`self.BP_BuildingComponent`)))
        (:`Is Not Valid`
          (`KismetSystemLibrary.PrintString` "NO IDEA"))))))

(fn `UserConstructionScript`
  (`parent.UserConstructionScript`))