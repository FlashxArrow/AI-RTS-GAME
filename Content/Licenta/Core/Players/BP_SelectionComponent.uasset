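; BP_SelectionComponent is an actor component that gives its owner a selection indicator decal and reports a team attitude.
; On BeginPlay it adds a scaled decal component beneath the owner with the selection indicator material, then hides it.
; Show and hide events toggle the decal's visibility and hidden-in-game state.
; GetTeamAttitude always returns Friendly.
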(event `self.ReceiveBeginPlay`
  (bind _returnvalue (`|AddComponentByClass` (`self.GetOwner`) "/Script/Engine.DecalComponent" false (`KismetMathLibrary.MakeTransform` (0.0 0.0 -70.0) (struct :`Pitch` 90.0) (`self.ScaleDecal`))))
  (set `self.DecalComponentRef` _returnvalue)
  (`DecalComponent.SetDecalMaterial` (`self.DecalComponentRef`) "/Game/Licenta/Core/Players/MI_SelectionIndicator.MI_SelectionIndicator")
  (`self.HideSelectionDecal`))

(event `ShowSelectionDecal`
  (bind _decalcomponentref (`self.DecalComponentRef`))
  (`SceneComponent.SetVisibility` _decalcomponentref true false)
  (`SceneComponent.SetHiddenInGame` _decalcomponentref false false))

(event `HideSelectionDecal`
  (bind _decalcomponentref (`self.DecalComponentRef`))
  (`SceneComponent.SetVisibility` _decalcomponentref false false)
  (`SceneComponent.SetHiddenInGame` _decalcomponentref true false))

(fn `GetTeamAttitude`
  (returns (TeamAttitude :type "ETeamAttitude Enum"))
  (return "Friendly"))