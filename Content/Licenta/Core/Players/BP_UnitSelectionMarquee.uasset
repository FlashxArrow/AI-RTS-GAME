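; Drag-selection marquee actor for the RTS player, selecting friendly units inside a world-space box.
; While resizing, Tick stretches a tall collision box from the actor's location to the cursor hit and updates the HUD widget's marquee.
; Box overlaps send select and deselect interface messages to the player controller.
; Start/End functions toggle collision and HUD drawing; separate events handle click selection and clearing of SelectedUnits.
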(event `self.ReceiveTick`
  (params (DeltaSeconds :type "Float (single-precision)"))
  (bind (_returnvalue_x _returnvalue_y) (`KismetMathLibrary.BreakVector` (/ (`KismetMathLibrary.Vector_GetAbs` (- (`self.K2_GetActorLocation`) (`self.EndMouseLocation`))) 2.0)))
  (if (`self.ShouldResizeMarquee`)
    (bind _aspc_rts_game (cast `/Game/Licenta/Core/Players/PC_RTS_GAME` (`GameplayStatics.GetPlayerController` 0)))
    (set `self.EndMouseLocation` (`.Location` (`GameplayStatics.BreakHitResult` (`PlayerController.GetHitResultUnderCursorByChannel` _aspc_rts_game "TraceTypeQuery1" true))))
    (`SceneComponent.K2_SetWorldLocation` (`self.BoxCol`) (`KismetMathLibrary.VLerp` (`self.K2_GetActorLocation`) (`self.EndMouseLocation`) 0.5) false false)
    (`BoxComponent.SetBoxExtent` (`self.BoxCol`) (`KismetMathLibrary.MakeVector` _returnvalue_x _returnvalue_y 300.0) true)
    (bind _asbp_hud (cast `/Game/Licenta/Core/Players/BP_HUD` (`PlayerController.GetHUD` (`GameplayStatics.GetPlayerController` 0))))
    (`/Game/Licenta/Core/UI/Menus/WBP_HUD.UpdateMarquee` (`/Game/Licenta/Core/Players/BP_HUD.HUDWidgetRef` _asbp_hud))))

(event `self.BoxCol.OnComponentBeginOverlap`
  (params (OverlappedComponent :type "PrimitiveComponent Object Reference") (OtherActor :type "Actor Object Reference") (OtherComp :type "PrimitiveComponent Object Reference") (OtherBodyIndex :type Integer) (bFromSweep :type Boolean) (SweepResult :type "HitResult Structure (by ref)"))
  (if (`KismetSystemLibrary.DoesImplementInterface` OtherActor "/Game/Licenta/Core/Buildings/BPI_SelectionEvents.BPI_SelectionEvents_C")
    (bind _teamattitude (message `/Game/Licenta/Core/Buildings/BPI_SelectionEvents.GetTeamAttitude` OtherActor))
    (if (`|EnumEquality` _teamattitude "Friendly")
      (message `/Game/Licenta/Core/Buildings/BPI_SelectionEvents.SelectThisActor` (`GameplayStatics.GetPlayerController` 0) OtherActor))
    (else
      (`KismetSystemLibrary.PrintString` "Not Selected"))))

(event `self.BoxCol.OnComponentEndOverlap`
  (params (OverlappedComponent :type "PrimitiveComponent Object Reference") (OtherActor :type "Actor Object Reference") (OtherComp :type "PrimitiveComponent Object Reference") (OtherBodyIndex :type Integer))
  (if (and (`self.ShouldResizeMarquee`) (`KismetSystemLibrary.DoesImplementInterface` OtherActor "/Game/Licenta/Core/Buildings/BPI_SelectionEvents.BPI_SelectionEvents_C"))
    (message `/Game/Licenta/Core/Buildings/BPI_SelectionEvents.DeselectThisActor` (`GameplayStatics.GetPlayerController` 0) OtherActor)))

(event `/Game/Licenta/Core/Buildings/BPI_SelectionEvents.ClearSelectedUnits`
  (bind _selectedunits (`self.SelectedUnits`))
  (for _array_element _selectedunits
    (message `/Game/Licenta/Core/Buildings/BPI_SelectionEvents.DeselectThisActor` (`GameplayStatics.GetPlayerController` 0) _array_element))
  (`KismetArrayLibrary.Array_Clear` _selectedunits))

(event `/Game/Licenta/Core/Buildings/BPI_SelectionEvents.SelectSingleUnit`
  (params (Unit :type "Actor Object Reference"))
  (message `/Game/Licenta/Core/Buildings/BPI_SelectionEvents.ClickSelectThisActor` (`GameplayStatics.GetPlayerController` 0) Unit)
  (`KismetArrayLibrary.Array_AddUnique` (`self.SelectedUnits`) Unit))

(fn `EndResizingMarquee`
  (set `self.ShouldResizeMarquee` false)
  (`PrimitiveComponent.SetCollisionEnabled` (`self.BoxCol`) "NoCollision")
  (bind _asbp_hud (cast `/Game/Licenta/Core/Players/BP_HUD` (`PlayerController.GetHUD` (`GameplayStatics.GetPlayerController` 0))))
  (`/Game/Licenta/Core/UI/Menus/WBP_HUD.StopMarqueeUpdate` (`/Game/Licenta/Core/Players/BP_HUD.HUDWidgetRef` _asbp_hud)))

(fn `GetTeamAttitude`
  (returns (TeamAttitude :type "ETeamAttitude Enum"))
  (return "Friendly"))

(fn `StartResizingMarquee`
  (set `self.ShouldResizeMarquee` true)
  (`PrimitiveComponent.SetCollisionEnabled` (`self.BoxCol`) "QueryOnly")
  (bind _asbp_hud (cast `/Game/Licenta/Core/Players/BP_HUD` (`PlayerController.GetHUD` (`GameplayStatics.GetPlayerController` 0))))
  (`/Game/Licenta/Core/UI/Menus/WBP_HUD.StartMarqueeUpdate` (`/Game/Licenta/Core/Players/BP_HUD.HUDWidgetRef` _asbp_hud)))

(fn `UserConstructionScript`)