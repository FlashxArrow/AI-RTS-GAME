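; BP_UNIT_SOLDIER is an RTS unit component that gives its owning actor health, team-based selection and unit state handling.
; On BeginPlay it adds a health bar widget colored by team attitude and binds the owner's click and damage events.
; Clicks add friendly units to PC_RTS_GAME's selection, while damage lowers clamped health and refreshes the bar.
; Worker and troop handlers store new states and fire enter-state calls; the tank handler is an empty stub.
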(event `self.ReceiveBeginPlay`
  (bind _returnvalue (`self.GetOwner`))
  (`|ExecutionSequence`
    (:`then_0`
      (`|ExecutionSequence`
        (:`then_0`
          (bind _returnvalue_2 (`|AddComponentByClass` _returnvalue "/Game/Licenta/Core/Players/BP_HealthBarWidget.BP_HealthBarWidget_C" false (`KismetMathLibrary.MakeTransform` (`self.HealthBarRelativeLocation`))))
          (`WidgetComponent.SetDrawSize` _returnvalue_2 (`self.HealthBarDrawSize`))
          (`/Game/Licenta/Core/Players/BP_HealthBarWidget.UpdateHealthBarColor` _returnvalue_2 (select `ETeamAttitude` (`self.TeamAttitude`) :`Friendly` (struct :`G` 0.5 :`B` 1.0 :`A` 1.0) :`Neutral` (struct :`R` 0.896513 :`G` 1.0 :`A` 1.0) :`Hostile` (struct :`R` 1.0 :`A` 1.0) :!type "LinearColor Structure"))
          (`self.UpdateHealthBar`))
        (:`then_1`
          (add `Actor.OnClicked` _returnvalue (`|CreateDelegate` :!event `OnOwnerClicked`))
          (add `Actor.OnTakeAnyDamage` (`self.GetOwner`) (`|CreateDelegate` :!event `OnOwnerTakeAnyDamage`)))))))

(event `OnOwnerClicked`
  (params (TouchedActor :type "Actor Object Reference") (ButtonPressed :type "Key Structure" :default "None"))
  (if (`|EnumEquality` (`self.TeamAttitude`) "Friendly")
    (`self.AddUnitToSelectionList`)))

(event `AddUnitToSelectionList`
  (bind _aspc_rts_game (cast `/Game/Licenta/Core/Players/PC_RTS_GAME` (`GameplayStatics.GetPlayerController` 0)))
  (`/Game/Licenta/Core/Players/PC_RTS_GAME.AddActorSelected` _aspc_rts_game (`self.GetOwner`)))

(event `OnOwnerTakeAnyDamage`
  (params (DamagedActor :type "Actor Object Reference") (Damage :type "Float (single-precision)") (DamageType :type "DamageType Object Reference") (InstigatedBy :type "Controller Object Reference") (DamageCauser :type "Actor Object Reference"))
  (set `self.Health` (`KismetMathLibrary.FMax` (- (`self.Health`) Damage)))
  (`self.UpdateHealthBar`))

(fn `HandleTankNewUnitState`
  (params (NewTankUnitState :type "/Game/Licenta/Core/Players/tank/E_TankUnitStates Enum" :default "NewEnumerator0")))

(fn `HandleTroopNewUnitState`
  (params (NewTroopUnitState :type "/Game/Licenta/Core/Players/Soldier/E_TroopUnitStates Enum" :default "NewEnumerator0"))
  (bind _output_get (set `self.TroopUnitState` NewTroopUnitState))
  (`self.OnEnterTroopState` _output_get))

(fn `HandleWorkerNewUnitState`
  (params (NewWorkerUnitState :type "/Game/Licenta/Core/Players/worker/E_WorkerUnitStates Enum" :default "NewEnumerator0"))
  (bind _output_get (set `self.WorkerUnitState` NewWorkerUnitState))
  (`self.OnEnterWorkerState` _output_get))

(fn `UpdateHealthBar`
  (bind _returnvalue (`Actor.GetComponentByClass` (`self.GetOwner`) "/Game/Licenta/Core/Players/BP_HealthBarWidget.BP_HealthBarWidget_C"))
  (`/Engine/EditorBlueprintResources/StandardMacros.IsValid` _returnvalue
    (:`Is Valid`
      (`/Game/Licenta/Core/Players/BP_HealthBarWidget.UpdateHealthBar` _returnvalue (/ (`self.Health`) (`self.HealthMax`))))
    (:`Is Not Valid`
      (`KismetSystemLibrary.LogString` "Unit doesn t have health bar"))))